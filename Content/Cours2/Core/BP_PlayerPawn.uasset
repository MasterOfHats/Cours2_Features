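; Player pawn with camera-relative movement, jumping, wall jumping and wallrunning, driven by a movement-state machine on SimplePawnMovement.
; Movement component events and per-tick wall traces select Walking, Jumping, Falling or Wallrun, which set gravity, capsule height and mesh tilt.
; A timeline buffers jump input, a delayed state copy gives coyote time, and wall jumps briefly lock move input.
; Tick also publishes player position to MPC_PawnData and prints the state for debugging.
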(event Custom|Handle_OnLanding
  ;[1 1 1] Initial values
  (MovementChange|ChangeMovementState "NewEnumerator0"))

(event Custom|Handle_OnFloorLeft
  ;[1 1 1] Initial values
  (if (Utilities|Enum|NotEqual(Enum) (Variables|MovementChange|GetMovementState) "NewEnumerator1")
    (MovementChange|ChangeMovementState "NewEnumerator2")))

(event Custom|Handle_OnApexReached
  ;[1 1 1] Initial values
  (if (Utilities|Enum|Equal(Enum) (Variables|MovementChange|GetMovementState) "NewEnumerator1")
    (MovementChange|ChangeMovementState "NewEnumerator2")))

(event Custom|StartJump
  (bind _simplepawnmovement (Variables|Default|GetSimplePawnMovement))
  (bind _wallnormal (Variables|Wall|GetWallNormal))
  (bind _walljumpstrength (Variables|Wall|GetWalljumpStrength))
  (bind _returnvalue (Class|KismetMathLibrary|VectorNormal2D _wallnormal 0.0001))
  (bind _returnvalue_2 (* _returnvalue _walljumpstrength))
  ;[0.25 0.25 0.25 0] Jump selection
  (if (Utilities|Enum|Equal(Enum) (Variables|MovementChange|GetCoyoteMovementState) "NewEnumerator0")
    (MovementChange|ChangeMovementState "NewEnumerator1")
    (Variables|/Script/Engine.MovementComponent|SetVelocity _simplepawnmovement (Math|Vector|MakeVector (.x (Variables|/Script/Engine.MovementComponent|GetVelocity _simplepawnmovement)) (.y (Variables|/Script/Engine.MovementComponent|GetVelocity _simplepawnmovement)) (Variables|Default|GetJumpZVel)))
    (elif (or (Utilities|Enum|Equal(Enum) (Variables|MovementChange|GetCoyoteMovementState) "NewEnumerator3") (Variables|Wall|GetbCanWallJump))
      (Variables|Wall|SetbCanWallJump false)
      (MovementChange|ChangeMovementState "NewEnumerator1")
      (Variables|/Script/Engine.MovementComponent|SetVelocity (Variables|Default|GetSimplePawnMovement) (Math|Vector|MakeVector (.x _returnvalue_2) (.y _returnvalue_2) (Variables|Default|GetJumpZVel)))
      (|DisablingInputsTemporarily))))

(event Custom|StopJumpBuffer
  (Utilities|FlowControl|Delay 0.0)
  (Timeline|JumpBuffer Stop
    (:Update
      (CallFunction|StartJump))))

(event Custom|WallHit
  (params (Hit :type Hit%20Result%20Structure))
  (bind _impactnormal (Collision|BreakHitResult Hit))
  ;[0.25 0.25 0.25 0] Wallrun logic
  (if (Utilities|Enum|NotEqual(Enum) (Variables|MovementChange|GetMovementState) "NewEnumerator0")
    (if (Wall|IsWallWalkable _impactnormal)
      (bind _returnvalue (Wall|IsWallTallEnough _impactnormal))
      (if _returnvalue
        (Variables|Wall|SetWallNormal _impactnormal)
        (Variables|Wall|SetWallrunDirection (Wall|GetWallrunDirection (Variables|Wall|GetWallNormal)))
        (MovementChange|ChangeMovementState "NewEnumerator3")))))

(event EventBeginPlay
  ;[1 1 1] Initial values
  (EventDispatchers|BindEventtoOnLanding (Variables|Default|GetSimplePawnMovement) (delegate Custom|Handle_OnLanding))
  (EventDispatchers|BindEventtoOnFloorLeft (Variables|Default|GetSimplePawnMovement) (delegate Custom|Handle_OnFloorLeft))
  (EventDispatchers|AssignOnApexReached (Variables|Default|GetSimplePawnMovement) (delegate Custom|Handle_OnApexReached))
  (Variables|Default|SetOriginalGravityAccel (Variables|/Script/Cours2.SimplePawnMovement|GetGravityAccel (Variables|Default|GetSimplePawnMovement))))

(event EventTick
  (params (DeltaSeconds :type Float%20%28single-precision%29))
  (Utilities|FlowControl|Sequence
    (:then_0
      (|RotateCapsuletoMovement)
      (|SetCollectionParamValues))
    (:then_1
      (CallFunction|DEBUGTick))
    (:then_2
      (if (Utilities|Enum|NotEqual(Enum) (Variables|MovementChange|GetMovementState) "NewEnumerator3")
        (bind (_returnvalue _normal _outhit) (Wall|CheckifGrazingWall 5.0))
        (if _returnvalue
          (Variables|Wall|SetbCanWallJump true)
          (Variables|Wall|SetWallNormal _normal)
          (if (Utilities|Enum|NotEqual(Enum) (Variables|MovementChange|GetMovementState) "NewEnumerator1")
            (CallFunction|WallHit _outhit)))))
    (:then_3
      (if (Utilities|Enum|Equal(Enum) (Variables|MovementChange|GetMovementState) "NewEnumerator3")
        (|WallrunMovement)))))

(event Input|ActionEvents|InputActionInputJump
  (params (Key :type Key%20Structure :default "None"))
  (:Pressed
    (Timeline|JumpBuffer PlayFromStart
      (:Update
        (CallFunction|StartJump)))))

(event Input|AxisEvents|InputAxisMoveForward
  (params (AxisValue :type Float%20%28single-precision%29))
  (if (not (Variables|Default|GetbIgnoreMoveInput))
    (switch Utilities|FlowControl|Switch|SwitchonEMovementState (Variables|MovementChange|GetMovementState)
      (:NewEnumerator0
        _)
      (:NewEnumerator1
        _)
      (:NewEnumerator2
        _))
    (Walking|MoveForwardGround (Input|AxisValues|GetMoveForward))))

(event Input|AxisEvents|InputAxisMoveRight
  (params (AxisValue :type Float%20%28single-precision%29))
  (if (not (Variables|Default|GetbIgnoreMoveInput))
    (switch Utilities|FlowControl|Switch|SwitchonEMovementState (Variables|MovementChange|GetMovementState)
      (:NewEnumerator0
        _)
      (:NewEnumerator1
        _)
      (:NewEnumerator2
        _))
    (Walking|MoveRightGround (Input|AxisValues|GetMoveRight))))

(event Input|AxisEvents|InputAxisCameraUp
  (params (AxisValue :type Float%20%28single-precision%29))
  (Pawn|Input|AddControllerPitchInput AxisValue))

(event Input|AxisEvents|InputAxisCameraRight
  (params (AxisValue :type Float%20%28single-precision%29))
  (Pawn|Input|AddControllerYawInput AxisValue))

(fn ConstructionScript)

(fn GetXYVelocity
  (return (* (Transformation|GetVelocity) "1.000000,1.000000, 0")))

(fn ChangeMovementState
  (params (NewMovementState :type EMovementState%20Enum :default "NewEnumerator0"))
  (bind _simplepawnmovement (Variables|Default|GetSimplePawnMovement))
  (LocalVariables|SetOldMovementState (Variables|MovementChange|GetMovementState))
  (bind _output_get (Variables|MovementChange|SetMovementState NewMovementState))
  (if (Utilities|Enum|NotEqual(Enum) (Variables|MovementChange|GetMovementState) (LocalVariables|GetOldMovementState))
    (Utilities|FlowControl|Sequence
      (:then_0
        ;[0.25 0.25 0.25 0] On entering movement state
        (switch Utilities|FlowControl|Switch|SwitchonEMovementState _output_get
          (:NewEnumerator0
            (Variables|/Script/Cours2.SimplePawnMovement|SetbActiveGravity (Variables|Default|GetSimplePawnMovement) false))
          (:NewEnumerator1
            (Variables|/Script/Cours2.SimplePawnMovement|SetbActiveGravity (Variables|Default|GetSimplePawnMovement) true)
            (Components|Capsule|SetCapsuleHalfHeight (Variables|Default|GetCapsule) 3e+01 true)
            (CallFunction|StopJumpBuffer)
            (Variables|/Script/Cours2.SimplePawnMovement|SetGravityAccel (Variables|Default|GetSimplePawnMovement) 2.5e+03))
          (:NewEnumerator2
            (Variables|/Script/Cours2.SimplePawnMovement|SetbActiveGravity (Variables|Default|GetSimplePawnMovement) true)
            (Variables|/Script/Cours2.SimplePawnMovement|SetGravityAccel (Variables|Default|GetSimplePawnMovement) (Variables|Default|GetOriginalGravityAccel)))
          (:NewEnumerator3
            (Wall|SetWallRunCosmetic (Variables|Wall|GetWallNormal))
            (Variables|/Script/Cours2.SimplePawnMovement|SetbActiveGravity (Variables|Default|GetSimplePawnMovement) false)
            (Variables|/Script/Engine.MovementComponent|SetVelocity _simplepawnmovement (* (Variables|/Script/Engine.MovementComponent|GetVelocity _simplepawnmovement) "1.000000,1.000000, 0")))))
      (:then_1
        ;[0.25 0.25 0.25 0] On exiting movement functionality
        (switch Utilities|FlowControl|Switch|SwitchonEMovementState (LocalVariables|GetOldMovementState)
          (:NewEnumerator0
            (Utilities|Time|SetTimerbyFunctionName 0 "ChangeCoyoteMovementState" (Variables|MovementChange|GetCoyoteTime)))
          (:NewEnumerator1
            (Components|Capsule|SetCapsuleHalfHeight (Variables|Default|GetCapsule) 85.0 true)
            (MovementChange|ChangeCoyoteMovementState))
          (:NewEnumerator2
            (MovementChange|ChangeCoyoteMovementState))
          (:NewEnumerator3
            (Wall|ResetCosmeticLocation)
            (Utilities|Time|SetTimerbyFunctionName 0 "ChangeCoyoteMovementState" (Variables|MovementChange|GetCoyoteTime))))))
    (else
      (return))))

(fn MoveForwardGround
  (params (AxisValue :type Float%20%28single-precision%29))
  (Pawn|Input|AddMovementInput (Class|KismetMathLibrary|VectorNormal2D (Math|Vector|GetForwardVector (Pawn|GetControlRotation :!class /Script/Engine.Pawn)) 0.0001) (* AxisValue (Variables|Walking|GetMoveAccel)) false))

(fn MoveRightGround
  (params (AxisValue :type Float%20%28single-precision%29))
  (Pawn|Input|AddMovementInput (Walking|GetGroundForward) (* AxisValue (Variables|Walking|GetMoveAccel)) false))

(fn GetGroundForward
  (return (Class|KismetMathLibrary|VectorNormal2D (Math|Vector|GetRightVector (Pawn|GetControlRotation :!class /Script/Engine.Pawn)) 0.0001)))

(fn CheckifGrazingWall
  (params (ExtraRadius :type Float%20%28single-precision%29))
  (bind _returnvalue (Transformation|GetActorLocation))
  (bind _capsule (Variables|Default|GetCapsule))
  (bind _returnvalue_2 (Components|Capsule|GetScaledCapsuleHalfHeight _capsule))
  (bind (_outhit _returnvalue_3) (Collision|SphereTraceForObjects (- _returnvalue (Math|Vector|MakeVector 0.0 0.0 _returnvalue_2)) (+ _returnvalue (Math|Vector|MakeVector 0.0 0.0 _returnvalue_2)) (+ (Components|Capsule|GetScaledCapsuleRadius (Variables|Default|GetCapsule)) ExtraRadius) (Variables|Wall|GetWallObjects) false 0 "None"))
  (if _returnvalue_3
    (if (Wall|IsWallStraight (.ImpactNormal (Collision|BreakHitResult _outhit)))
      (return (Wall|IsWallStraight (.ImpactNormal (Collision|BreakHitResult _outhit))) (.ImpactNormal (Collision|BreakHitResult _outhit)) _outhit))))

(fn IsWallStraight
  (params (Normal :type Vector))
  (return (< (Math|Float|Absolute(Float) (Math|Vector|DotProduct Normal "0, 0,1.000000")) 0.3)))

(fn DEBUGTick
  (Development|PrintString (Utilities|String|EnumtoString (Variables|MovementChange|GetMovementState)) true true "(R=0.515625,G=0.147588,B=0.012459,A=1.000000)" 0.0))

(fn StopVelZ
  (bind _returnvalue (Transformation|GetVelocity))
  (Variables|/Script/Engine.MovementComponent|SetVelocity (Variables|Default|GetSimplePawnMovement) (Math|Vector|MakeVector (.x _returnvalue) (.y _returnvalue) 0.0)))

(fn SetWallRunCosmetic
  (params (WallNormal :type Vector))
  (bind _capsule (Variables|Default|GetCapsule))
  (bind _returnvalue (Math|Vector|GetRightVector _capsule))
  (bind _returnvalue_2 (Math|Vector|DotProduct WallNormal _returnvalue))
  (bind _returnvalue_3 (Math|Float|Sign(Float) _returnvalue_2))
  (Transformation|SetRelativeRotation (Variables|Default|GetSkeletalMesh) (Math|Rotator|MakeRotator 0.0 (* 3e+01 _returnvalue_3) -9e+01) false false)
  (Transformation|SetRelativeLocation (Variables|Default|GetSkeletalMesh) (Math|Vector|MakeVector 0.0 (* -2e+01 _returnvalue_3) -9e+01) false false))

(fn ResetCosmeticLocation
  (Transformation|SetRelativeRotation (Variables|Default|GetSkeletalMesh) (Math|Rotator|MakeRotator 0.0 0.0 -9e+01) false false)
  (Transformation|SetRelativeLocation (Variables|Default|GetSkeletalMesh) (Math|Vector|MakeVector 0.0 0.0 -9e+01) false false))

(fn ChangeCoyoteMovementState
  (Variables|MovementChange|SetCoyoteMovementState (Variables|MovementChange|GetMovementState)))

(fn IsWallWalkable
  (params (Normal :type Vector))
  (return (and (Wall|IsWallStraight Normal) (or (< (Math|Float|Absolute(Float) (Math|Vector|DotProduct Normal (Class|KismetMathLibrary|VectorNormal2D (Pawn|Components|PawnMovement|GetLastInputVector (Variables|Default|GetSimplePawnMovement)) 0.0001))) 0.86) (and (Math|Vector|Equal(Vector) (* (Pawn|Components|PawnMovement|GetLastInputVector (Variables|Default|GetSimplePawnMovement)) "1.000000,1.000000, 0") "0, 0, 0" 0.0001) (< (Math|Vector|DotProduct Normal (Class|KismetMathLibrary|VectorNormal2D (Math|Vector|GetForwardVector (Pawn|GetControlRotation :!class /Script/Engine.Pawn)) 0.0001)) 0.7))))))

(fn IsWallTallEnough
  (params (Normal :type Vector))
  (Utilities|FlowControl|Sequence
    (:then_0
      (LocalVariables|SetLocalNormal Normal)
      (for _index (range 0 1)
        (bind (_outhit _returnvalue) (Collision|LineTraceForObjects (+ (Transformation|GetActorLocation) (Math|Vector|MakeVector 0.0 0.0 (* (Utilities|Select :Index _index :Option%200 0.0 :Option%201 1.0) (Variables|/Script/Engine.CapsuleComponent|GetCapsuleHalfHeight (Variables|Default|GetCapsule))))) (+ (+ (Transformation|GetActorLocation) (Math|Vector|MakeVector 0.0 0.0 (* (Utilities|Select :Index _index :Option%200 0.0 :Option%201 1.0) (Variables|/Script/Engine.CapsuleComponent|GetCapsuleHalfHeight (Variables|Default|GetCapsule))))) (* Normal -5e+01)) (Variables|Wall|GetWallObjects) false 0 "None"))
        (if _returnvalue
          (if (not (Math|Vector|Equal(Vector) (.ImpactNormal (Collision|BreakHitResult _outhit)) (LocalVariables|GetLocalNormal) 0.0001))
            (return false))
          (else
            (return false)))))
    (:then_1
      (return true))))

(fn GetWallrunDirection
  (params (Normal :type Vector))
  (bind _returnvalue (Math|Vector|CrossProduct Normal "0, 0,1.000000"))
  (return (* (Math|Vector|Normalize _returnvalue) (Math|Float|Sign(Float) (Math|Vector|DotProduct _returnvalue (* (Variables|/Script/Engine.MovementComponent|GetVelocity (Variables|Default|GetSimplePawnMovement)) "1.000000,1.000000, 0"))))))

(fn ExitWallrun
  (if (Utilities|Enum|Equal(Enum) (Variables|MovementChange|GetMovementState) "NewEnumerator3")
    (MovementChange|ChangeMovementState "NewEnumerator2")))